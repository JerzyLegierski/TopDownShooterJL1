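; Spider enemy actor that chases the player character and plays attack animations.
; BeginPlay starts a loop that reissues an AI MoveTo toward the player every 0.2 seconds.
; Tick plays a montage when the range check passes and Spiderattack1 is not already playing.
; The range check passes at or beyond AttackDistance, not within it.
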(event `self.ReceiveBeginPlay`
  (`|AIMoveTo` self (0.0 0.0 0.0) (`GameplayStatics.GetPlayerCharacter` 0) :!label _label
    (:`then`
      (`KismetSystemLibrary.Delay` 0.2)
      (goto _label))))

(event `self.ReceiveTick`
  (params (DeltaSeconds :type "Float (single-precision)"))
  (if (`self.isattackrange`)
    (if (not (`self.isattacking`))
      (`|PlayMontage` (`self.Mesh`)))))

(fn `isattacking`
  (returns (NewParam :type Boolean))
  (return (`AnimInstance.Montage_IsPlaying` (`SkeletalMeshComponent.GetAnimInstance` (`self.Mesh`)) "/Game/Characters/Enemy_Great_Spider/Animations/spiderattack1.spiderattack1")))

(fn `isattackrange`
  (returns (NewParam :type Boolean))
  (return (>= (`self.GetDistanceTo` (`GameplayStatics.GetPlayerCharacter` 0)) (`self.attack distance`))))

(fn `UserConstructionScript`)
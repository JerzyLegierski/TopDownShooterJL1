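; Player soldier pawn that moves along fixed world X and Y axes, turns with the mouse and fires an assault rifle.
; Each tick, horizontal mouse velocity above a dead zone interpolates control rotation toward a yaw from Atan2; with vertical input zeroed, that target is only ±90 degrees.
; Firing is effects-only here: press activates the muzzle flash and loop sound, release stops both and plays a shot-end cue.
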(event `self.ReceiveTick`
  (params (DeltaSeconds :type "Float (single-precision)"))
  ;[1 1 1] Rotation
  (`self.updateplayerrotation`))

(event `InputAxis|moveforwardback`
  (params (AxisValue :type "Float (single-precision)"))
  ;[1 1 1] Movement
  (`self.AddMovementInput` (1.0 0.0 0.0) AxisValue))

(event `InputAxis|moveleftright`
  (params (AxisValue :type "Float (single-precision)"))
  ;[1 1 1] Movement
  (`self.AddMovementInput` (0.0 1.0 0.0) AxisValue))

(event `InputAction|Weaponfire`
  (params (Key :type "Key Structure"))
  ;[1 1 1] Firing weapon
  (:`Pressed`
    (`self.startfiringweapon`))
  (:`Released`
    (`self.stopfiringweapon`)))

(fn `getmousevelocity`
  (returns (NewParam :type "Vector2D Structure"))
  (return (/ (`KismetMathLibrary.MakeVector2D` (`PlayerController.GetInputMouseDelta` (`GameplayStatics.GetPlayerController` 0))) (`GameplayStatics.GetWorldDeltaSeconds`))))

(fn `ismouseabovedeadzone`
  (returns (NewParam :type Boolean))
  (return (> (`KismetMathLibrary.VSize2D` (`self.getmousevelocity`)) (`self.mousedeadzone`))))

(fn `startfiringweapon`
  (`ActorComponent.Activate` (`self.P_AssaultRifle_MF`) false)
  (bind _returnvalue (`GameplayStatics.SpawnSound2D` "/Game/Sounds/Weapon_AssaultRifle/Stereo/randomfireloop.randomfireloop" 1.0 1.0 0.0 null))
  (set `self.weaponfiresound` _returnvalue))

(fn `stopfiringweapon`
  (`ActorComponent.Deactivate` (`self.P_AssaultRifle_MF`))
  (`AudioComponent.Stop` (`self.weaponfiresound`))
  (`GameplayStatics.SpawnSound2D` "/Game/Sounds/Weapon_AssaultRifle/Stereo/shotendcue.shotendcue" 1.0 1.0 0.0 null))

(fn `updateplayerrotation`
  (bind _returnvalue (`GameplayStatics.GetPlayerController` 0))
  (bind (_newparam_x _newparam_y) (`KismetMathLibrary.BreakVector2D` (`self.getmousevelocity`)))
  (if (`self.ismouseabovedeadzone`)
    (`Controller.SetControlRotation` _returnvalue (`KismetMathLibrary.RInterpTo` (`Controller.GetControlRotation` _returnvalue) (`KismetMathLibrary.MakeRotator` 0.0 0.0 (`KismetMathLibrary.DegAtan2` _newparam_x _newparam_y)) (`GameplayStatics.GetWorldDeltaSeconds`) (`self.delta time multiply`)))))

(fn `UserConstructionScript`)